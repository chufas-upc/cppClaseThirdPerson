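; Character Blueprint that sets up the player's HUD and Steam name display, and triggers interactions on overlap.
; BeginPlay adds the HUD to the viewport and feeds the player's net ID to a username widget shown on its Widget component.
; Overlapped actors receive an OnInteract message, and debug Escape quits the game.
; PlayTurn plays montages gated by a Turning flag, while the 90-degree turn events are empty.
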(event Custom|PlayTurn
  (params (MontageToPlay :type Anim%20Montage%20Object%20Reference) (PlayRate :type Float%20%28single-precision%29))
  (if (Variables|Default|GetTurning)
    (Variables|Default|SetTurning true)
    (Animation|Montage|PlayMontage (Variables|Character|GetMesh) MontageToPlay PlayRate
      (:OnCompleted
        (Variables|Default|SetTurning false)))))

(event Custom|TurnLeft90)

(event Custom|TurnRight90)

(event EventBeginPlay
  (|CallParentFunction)
  (Development|PrintString "Hola" true true "(R=0.000000,G=0.660000,B=1.000000,A=1.000000)" 1e+01)
  (bind _returnvalue (UserInterface|CreateWidget "/Game/UI/WBP_HUD.WBP_HUD_C"))
  (UserInterface|Viewport|AddtoViewport _returnvalue 0)
  (bind _returnvalue_2 (UserInterface|CreateWidget "/Game/UI/WBP_UserName.WBP_UserName_C"))
  (Default|GatherSteamInfo _returnvalue_2 (Class|AdvancedSessionsLibrary|GetUniqueNetID (Game|GetPlayerController 0)))
  (UserInterface|SetWidget (Variables|Default|GetWidget) _returnvalue_2))

(event Collision|EventActorBeginOverlap
  (params (OtherActor :type Actor%20Object%20Reference))
  (Class|BPIInteractuable|OnInteract(Message) OtherActor self))

(event EventTick
  (params (DeltaSeconds :type Float%20%28single-precision%29)))

(event Input|KeyboardEvents|DebugKeyEscape
  (params (Key :type Key%20Structure :default "None") (ActionValue :type Input%20Action%20Value%20Structure))
  (:Released
    (Game|QuitGame 0 "Quit" false)))

(fn ConstructionScript
  (|CallParentFunction))