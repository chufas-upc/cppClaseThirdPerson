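; BP_Puerta is an interactable door that unlocks when the key in its level is collected.
; On BeginPlay it binds UnlockDoor to the KeyInLevel reference's key-collected event, which clears IsLocked.
; While unlocked, each Interact instantly rotates the root component a quarter turn, using IsClosed to pick the direction and then flipping that flag.
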(event `self.ReceiveBeginPlay`
  (add `/Game/Blueprints/Entrega1/BP_Llave.KeyCollected` (`self.KeyInLevel`) (delegate `UnlockDoor`)))

(event `UnlockDoor`
  (set `self.IsLocked` false))

(event `self.Interact`
  (params (player :type "Character Object Reference"))
  (if (not (`self.IsLocked`))
    (`SceneComponent.K2_AddLocalRotation` (`self.DefaultSceneRoot`) (`KismetMathLibrary.SelectRotator` (struct :`Yaw` -90.0) (struct :`Yaw` 90.0) (`self.IsClosed`)) false false)
    (set `self.IsClosed` (not (`self.IsClosed`)))))

(fn `UserConstructionScript`)