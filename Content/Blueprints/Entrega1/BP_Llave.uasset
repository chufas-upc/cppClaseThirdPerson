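; BP_Llave is a level key that stays hidden and non-interactable until every key fragment in the level has been collected.
; On BeginPlay it disables itself, then counts all BP_ItemFragmentLlave actors and binds to their collected events.
; Each collected fragment decrements the counter; at zero the mesh becomes visible and sphere collision switches to query-only.
; Interacting with it calls CallKeyCollected and destroys the actor.
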(event `self.ReceiveBeginPlay`
  (`|ExecutionSequence`
    (:`then_0`
      (`self.DesactivarLlave`))
    (:`then_1`
      (bind _outactors (`GameplayStatics.GetAllActorsOfClass` "/Game/Blueprints/Entrega1/BP_ItemFragmentLlave.BP_ItemFragmentLlave_C"))
      (for _array_element _outactors
        (add `/Game/Blueprints/Entrega1/BP_ItemFragmentLlave.FragmentoRecolectado` _array_element (delegate `RestarFragmento`))
        (`/Engine/EditorBlueprintResources/StandardMacros.IncrementInt` (`self.FragmentosNivel`))))))

(event `RestarFragmento`
  (bind _result (`/Engine/EditorBlueprintResources/StandardMacros.DecrementInt` (`self.FragmentosNivel`))
    (:`  `
      (if (<= _result 0)
        (`self.ActivarLlave`)))))

(event `self.Interact`
  (params (player :type "Character Object Reference"))
  (`self.KeyCollected`)
  (`self.K2_DestroyActor`))

(fn `ActivarLlave`
  (`SceneComponent.SetVisibility` (`self.Mesh`) true false)
  (`PrimitiveComponent.SetCollisionEnabled` (`self.SphereCollision`) "QueryOnly"))

(fn `DesactivarLlave`
  (`SceneComponent.SetVisibility` (`self.Mesh`) false false)
  (`PrimitiveComponent.SetCollisionEnabled` (`self.SphereCollision`) "NoCollision"))

(fn `UserConstructionScript`)