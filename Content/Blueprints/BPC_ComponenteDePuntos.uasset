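; Points component that provides functions for adding and subtracting points (Puntos).
; SumarPuntos and RestarPuntos each update Puntos with the matching arithmetic, then print a Spanish confirmation with the value, green for addition and red for subtraction.
; BeginPlay and Tick are empty, so the component does nothing until one of these functions is called.
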(fn `RestarPuntos`
  (params (Puntos :type Integer))
  (bind _output_get (set `self.Puntos` (- (`self.Puntos`) Puntos)))
  (`KismetSystemLibrary.PrintString` (`KismetStringLibrary.Concat_StrStr` "Se ha restado! Puntos: " (`KismetStringLibrary.Conv_IntToString` _output_get)) true true (struct :`R` 1.0 :`A` 1.0)))

(fn `SumarPuntos`
  (params (Puntos :type Integer))
  (bind _output_get (set `self.Puntos` (+ Puntos (`self.Puntos`))))
  (`KismetSystemLibrary.PrintString` (`KismetStringLibrary.Concat_StrStr` "Se ha sumado! Puntos: " (`KismetStringLibrary.Conv_IntToString` _output_get)) true true (struct :`R` 0.112148 :`G` 1.0 :`A` 1.0)))