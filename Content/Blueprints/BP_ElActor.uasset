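; BP_ElActor is an actor that shows the local player's Steam avatar on its Plane mesh.
; On BeginPlay it requests the large Steam avatar for the first player controller's unique net ID.
; Success creates a dynamic M_Texture material instance and feeds the avatar into its SpriteTexture parameter, while failure prints an error.
; An image-download path and a decal material call remain as unconnected leftovers that never run.
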(event `self.ReceiveBeginPlay`
  (bind _returnvalue (`AdvancedSteamFriendsLibrary.GetSteamFriendAvatar` (`AdvancedSessionsLibrary.GetUniqueNetID` (`GameplayStatics.GetPlayerController` 0)) "SteamAvatar_Large")
    (:`OnSuccess`
      (bind _returnvalue_2 (`PrimitiveComponent.CreateDynamicMaterialInstance` (`self.Plane`) 0 "/Game/Mats/M_Texture.M_Texture" "SpriteTexture"))
      (`MaterialInstanceDynamic.SetTextureParameterValue` _returnvalue_2 "SpriteTexture" _returnvalue))
    (:`OnFailure`
      (`KismetSystemLibrary.PrintString` (`KismetStringLibrary.Concat_StrStr` "Error: " (`KismetSystemLibrary.GetDisplayName` _returnvalue)) true true (struct :`G` 0.66 :`B` 1.0 :`A` 1.0) 10.0))))

(event `self.ReceiveTick`
  (params (DeltaSeconds :type "Float (single-precision)")))

(fn `UserConstructionScript`)