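; Actor Blueprint for the HuTao character model that publishes its head orientation to materials.
; Every Tick, it reads the world-space transform of the head bone ("頭") on HutaoModelTransform.
; It writes that bone's forward, right and up vectors to the MPC_Light parameter collection as HeadFoward (spelled that way), HeadRight and HeadUp.
; BeginPlay, overlap and the construction script do nothing.
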(event `self.ReceiveTick`
  (params (DeltaSeconds :type "Float (single-precision)"))
  (bind (_returnvalue_location _returnvalue_rotation) (`KismetMathLibrary.BreakTransform` (`SkinnedMeshComponent.GetBoneTransform` (`self.hutao_model_transform`) "頭" "RTS_World")))
  (`KismetMaterialLibrary.SetVectorParameterValue` "/Game/External/HuTao/tex/MPC_Light.MPC_Light" "HeadFoward" (`KismetMathLibrary.Conv_VectorToLinearColor` (`KismetMathLibrary.GetForwardVector` _returnvalue_rotation)))
  (`KismetMaterialLibrary.SetVectorParameterValue` "/Game/External/HuTao/tex/MPC_Light.MPC_Light" "HeadRight" (`KismetMathLibrary.Conv_VectorToLinearColor` (`KismetMathLibrary.GetRightVector` _returnvalue_rotation)))
  (`KismetMaterialLibrary.SetVectorParameterValue` "/Game/External/HuTao/tex/MPC_Light.MPC_Light" "HeadUp" (`KismetMathLibrary.Conv_VectorToLinearColor` (`KismetMathLibrary.GetUpVector` _returnvalue_rotation))))

(fn `UserConstructionScript`)